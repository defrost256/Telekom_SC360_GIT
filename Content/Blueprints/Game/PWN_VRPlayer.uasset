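; VR player pawn that lights up the controls on its Oculus controller hand meshes as they are used.
; BeginPlay creates a dynamic material instance for each hand mesh and sets floor-level tracking origin.
; Grip and trigger axes scale glow parameters on the matching hand, while face buttons switch glow between maximum and zero.
; Right-hand face buttons write to the left-hand material, just like the left-hand ones.
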(event `self.ReceiveBeginPlay`
  (bind _returnvalue (`PrimitiveComponent.CreateDynamicMaterialInstance` (`self.RightHandMesh`) 0 "/Game/BaseMaterials/Placeholder/MI_OculusController.MI_OculusController"))
  (set `self.RightHandMaterial` _returnvalue)
  (bind _returnvalue_2 (`PrimitiveComponent.CreateDynamicMaterialInstance` (`self.LeftHandMesh`) 0 "/Game/BaseMaterials/Placeholder/MI_OculusController.MI_OculusController"))
  (set `self.LeftHandMaterial` _returnvalue_2)
  (`HeadMountedDisplayFunctionLibrary.SetTrackingOrigin` "Floor"))

(event `InputAxisKey|MotionController_Left_Grip1Axis`
  (params (AxisValue :type "Float (single-precision)"))
  (`MaterialInstanceDynamic.SetScalarParameterValue` (`self.LeftHandMaterial`) (`KismetStringLibrary.Conv_StringToName` (`self.GripMatParam`)) (* AxisValue (`self.ButtonGlowMax`))))

(event `InputAxisKey|MotionController_Right_Grip1Axis`
  (params (AxisValue :type "Float (single-precision)"))
  (`MaterialInstanceDynamic.SetScalarParameterValue` (`self.RightHandMaterial`) (`KismetStringLibrary.Conv_StringToName` (`self.GripMatParam`)) (* (`self.ButtonGlowMax`) AxisValue)))

(event `InputAxisKey|MotionController_Left_TriggerAxis`
  (params (AxisValue :type "Float (single-precision)"))
  (`MaterialInstanceDynamic.SetScalarParameterValue` (`self.LeftHandMaterial`) (`KismetStringLibrary.Conv_StringToName` (`self.TriggerMatParam`)) (* AxisValue (`self.ButtonGlowMax`))))

(event `InputAxisKey|MotionController_Right_TriggerAxis`
  (params (AxisValue :type "Float (single-precision)"))
  (`MaterialInstanceDynamic.SetScalarParameterValue` (`self.RightHandMaterial`) (`KismetStringLibrary.Conv_StringToName` (`self.TriggerMatParam`)) (* (`self.ButtonGlowMax`) AxisValue)))

(event `Key|MotionController_Left_FaceButton1`
  (params (Key :type "Key Structure"))
  (bind _lefthandmaterial (`self.LeftHandMaterial`))
  (bind _returnvalue (`KismetStringLibrary.Conv_StringToName` (`self.TopButtonMatParam`)))
  (:`Pressed`
    (`MaterialInstanceDynamic.SetScalarParameterValue` _lefthandmaterial _returnvalue (`self.ButtonGlowMax`)))
  (:`Released`
    (`MaterialInstanceDynamic.SetScalarParameterValue` _lefthandmaterial _returnvalue 0.0)))

(event `Key|MotionController_Left_FaceButton2`
  (params (Key :type "Key Structure"))
  (bind _lefthandmaterial (`self.LeftHandMaterial`))
  (bind _returnvalue (`KismetStringLibrary.Conv_StringToName` (`self.BottomButtonMatParam`)))
  (:`Pressed`
    (`MaterialInstanceDynamic.SetScalarParameterValue` _lefthandmaterial _returnvalue (`self.ButtonGlowMax`)))
  (:`Released`
    (`MaterialInstanceDynamic.SetScalarParameterValue` _lefthandmaterial _returnvalue 0.0)))

(event `Key|MotionController_Right_FaceButton1`
  (params (Key :type "Key Structure"))
  (bind _lefthandmaterial (`self.LeftHandMaterial`))
  (bind _returnvalue (`KismetStringLibrary.Conv_StringToName` (`self.TopButtonMatParam`)))
  (:`Pressed`
    (`MaterialInstanceDynamic.SetScalarParameterValue` _lefthandmaterial _returnvalue (`self.ButtonGlowMax`)))
  (:`Released`
    (`MaterialInstanceDynamic.SetScalarParameterValue` _lefthandmaterial _returnvalue 0.0)))

(event `Key|MotionController_Right_FaceButton2`
  (params (Key :type "Key Structure"))
  (bind _lefthandmaterial (`self.LeftHandMaterial`))
  (bind _returnvalue (`KismetStringLibrary.Conv_StringToName` (`self.BottomButtonMatParam`)))
  (:`Pressed`
    (`MaterialInstanceDynamic.SetScalarParameterValue` _lefthandmaterial _returnvalue (`self.ButtonGlowMax`)))
  (:`Released`
    (`MaterialInstanceDynamic.SetScalarParameterValue` _lefthandmaterial _returnvalue 0.0)))

(fn `UserConstructionScript`)