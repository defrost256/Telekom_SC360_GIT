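; BP_CarTest is a traffic car Blueprint that adds debug visualisation to inherited or external driving logic.
; After each traffic tick it calls DrawDebug, which runs only when DebugDraw is enabled.
; It prints the car's time and the road's desired speed for that time and car ID above it, and outlines the sensing area when the path is not free.
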(event `self.AfterTrafficTick`
  (params (DeltaT :type "Float (single-precision)"))
  (`self.DrawDebug`))

(fn `DrawDebug`
  (bind _time (`self.time`))
  (bind _sensingarea (`self.sensingArea`))
  (if (`self.debugDraw`)
    (`|ExecutionSequence`
      (:`then_0`
        (`KismetSystemLibrary.DrawDebugString` (0.0 0.0 100.0) (`KismetStringLibrary.Concat_StrStr` (`KismetStringLibrary.Conv_DoubleToString` _time) " (" (`KismetStringLibrary.Conv_DoubleToString` (`TrafficRoad.GetDesiredSpeed` (`self.road`) _time (`self.GetUniqueID_Int`))) ")") self (struct :`R` 0.359375 :`G` 0.359375 :`B` 0.359375 :`A` 1.0)))
      (:`then_1`
        (if (not (`self.freePath`))
          (`KismetSystemLibrary.DrawDebugBox` (`SceneComponent.K2_GetComponentLocation` _sensingarea) (`BoxComponent.BoxExtent` _sensingarea) (struct) (`SceneComponent.K2_GetComponentRotation` _sensingarea)))))))

(fn `UserConstructionScript`)