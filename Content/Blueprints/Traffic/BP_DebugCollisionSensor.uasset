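; Debug Blueprint in the Traffic folder that visualizes an actor's collision sensors every Tick, gated by three debug toggles.
; Activation debug boxes the current slowdown sensor with its overlap count and the emergency sensor when overlapped.
; Current-sensor debug boxes and prints that sensor's transform, while angle debug draws yaw-relative arcs for front, front-side, side and rear sectors.
; Tick also prints an unconditional "Hello", and no sensing logic lives in this graph.
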(event `self.ReceiveTick`
  (params (DeltaSeconds :type "Float (single-precision)"))
  (bind _returnvalue (`self.K2_GetActorLocation`))
  (bind _returnvalue_2 (`self.K2_GetActorLocation`))
  (bind _overlapcount (`self.overlapCount`))
  (bind _sideangle (`self.sideAngle`))
  (bind _frontsideangle (`self.frontSideAngle`))
  (bind _frontsideangle_2 (`self.frontSideAngle`))
  (bind _rearangle (`self.rearAngle`))
  (bind _emergencysensor (`self.EmergencySensor`))
  (bind _returnvalue_3 (- (`self.rearAngle`) _sideangle))
  (bind _yaw (.yaw (`self.K2_GetActorRotation`)))
  (bind _returnvalue_4 (- (`self.sideAngle`) _frontsideangle))
  (bind _yaw_2 (.yaw (`self.K2_GetActorRotation`)))
  (bind _returnvalue_5 (/ _returnvalue_3 360.0))
  (bind _returnvalue_6 (/ _returnvalue_4 360.0))
  (`KismetSystemLibrary.PrintString` "Hello")
  (`|ExecutionSequence`
    (:`then_0`
      (if (`self.bDebugSensorActivation`)
        (`|ExecutionSequence`
          (:`then_0`
            ;[1 1 1] SlowdownSensors
            (if (> _overlapcount 0)
              (bind _returnvalue_7 (`self.GetCurrentSensor`))
              (bind _returnvalue_8 (`SceneComponent.K2_GetComponentLocation` _returnvalue_7))
              (`KismetSystemLibrary.DrawDebugBox` _returnvalue_8 (`BoxComponent.BoxExtent` _returnvalue_7) (struct :`R` 1.0 :`G` 0.947471 :`A` 1.0) (`SceneComponent.K2_GetComponentRotation` _returnvalue_7))
              (`KismetSystemLibrary.DrawDebugString` _returnvalue_8 (`KismetStringLibrary.Conv_IntToString` _overlapcount) null (struct :`R` 0.868237 :`G` 1.0 :`A` 1.0))))
          (:`then_1`
            ;[1 1 1] Emergency Sensor
            (if (> (`self.emergencyOverlap`) 0)
              (`KismetSystemLibrary.DrawDebugBox` (`SceneComponent.K2_GetComponentLocation` _emergencysensor) (`BoxComponent.BoxExtent` _emergencysensor) (struct :`R` 1.0 :`B` 0.04747 :`A` 1.0) (`SceneComponent.K2_GetComponentRotation` _emergencysensor)))))))
    (:`then_1`
      (if (`self.bDebugCurrentSensor`)
        ;[1 1 1] CurrentSensor
        (bind _returnvalue_9 (`self.GetCurrentSensor`))
        (bind _returnvalue_10 (`SceneComponent.K2_GetComponentLocation` _returnvalue_9))
        (bind _returnvalue_11 (`SceneComponent.K2_GetComponentRotation` _returnvalue_9))
        (`KismetSystemLibrary.DrawDebugBox` _returnvalue_10 (`BoxComponent.BoxExtent` _returnvalue_9) (struct :`G` 1.0 :`B` 0.518557 :`A` 1.0) _returnvalue_11)
        (`KismetSystemLibrary.PrintString` (`KismetStringLibrary.Concat_StrStr` (`KismetStringLibrary.Conv_VectorToString` _returnvalue_10) "  " (`KismetStringLibrary.Conv_RotatorToString` _returnvalue_11)))))
    (:`then_2`
      (if (`self.bDebugSensorAngles`)
        (`|ExecutionSequence`
          (:`then_0`
            ;[1 1 1] Sensor Angles
            ;;[1 1 1] FrontSensorAngle
            (`EngineInterface_FL.DrawDebugArc` (`self.K2_GetActorLocation`) 250.0 (/ _frontsideangle_2 180.0) 10 (struct :`G` 1.0 :`A` 1.0) 0.0 0.0 (`KismetMathLibrary.MakeRotator` 0.0 90.0 (- (- (.yaw (`self.K2_GetActorRotation`)) _frontsideangle_2) 90.0))))
          (:`then_1`
            ;;[1 1 1] FrontSideSensorAngles
            (`|ExecutionSequence`
              (:`then_0`
                (`EngineInterface_FL.DrawDebugArc` _returnvalue_2 220.0 _returnvalue_6 10 (struct :`G` 1.0 :`B` 0.5 :`A` 1.0) 0.0 0.0 (`KismetMathLibrary.MakeRotator` 0.0 90.0 (+ _yaw_2 _frontsideangle -90.0))))
              (:`then_1`
                (`EngineInterface_FL.DrawDebugArc` _returnvalue_2 220.0 _returnvalue_6 10 (struct :`G` 1.0 :`B` 0.5 :`A` 1.0) 0.0 0.0 (`KismetMathLibrary.MakeRotator` 0.0 90.0 (- _yaw_2 (+ _returnvalue_4 _frontsideangle 90.0)))))))
          (:`then_2`
            ;;[1 1 1] SideSensorAngles
            (`|ExecutionSequence`
              (:`then_0`
                (`EngineInterface_FL.DrawDebugArc` _returnvalue 160.0 _returnvalue_5 10 (struct :`G` 0.683333 :`B` 1.0 :`A` 1.0) 0.0 0.0 (`KismetMathLibrary.MakeRotator` 0.0 90.0 (+ _yaw _sideangle -90.0))))
              (:`then_1`
                (`EngineInterface_FL.DrawDebugArc` _returnvalue 160.0 _returnvalue_5 10 (struct :`G` 0.683333 :`B` 1.0 :`A` 1.0) 0.0 0.0 (`KismetMathLibrary.MakeRotator` 0.0 90.0 (- _yaw (+ _returnvalue_3 _sideangle 90.0)))))))
          (:`then_3`
            ;;[1 1 1] RearSensorAngle
            (`EngineInterface_FL.DrawDebugArc` (`self.K2_GetActorLocation`) 190.0 (/ (- 180.0 _rearangle) 180.0) 10 (struct :`G` 0.167 :`B` 1.0 :`A` 1.0) 0.0 0.0 (`KismetMathLibrary.MakeRotator` 0.0 90.0 (+ (.yaw (`self.K2_GetActorRotation`)) _rearangle -90.0)))))))))

(fn `UserConstructionScript`)