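; Debug variant of a traffic raytrace sensor that visualizes its detection field and performs no traces itself.
; After the parent Tick, DebugAngles draws view-angle arcs centered on the actor's yaw at the emergency (red) and maximum (yellow) radii.
; DebugRays draws a yaw-stepped fan of lines, red to EmergencyRadius, then yellow to a point at MaxRadius minus EmergencyRadius from the actor, short of the outer arc.
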(event `self.ReceiveTick`
  (params (DeltaSeconds :type "Float (single-precision)"))
  (bind _returnvalue (`self.K2_GetActorLocation`))
  (bind _returnvalue_2 (/ (`self.viewAngle`) 360.0))
  (bind _returnvalue_3 (`KismetMathLibrary.MakeRotator` 0.0 90.0 (- (- (.yaw (`self.K2_GetActorRotation`)) (`self.halfAngle`)) 90.0)))
  (`parent.ReceiveTick` DeltaSeconds)
  (`|ExecutionSequence`
    (:`then_0`
      (if (`self.bDebugAngles`)
        (`|ExecutionSequence`
          (:`then_0`
            (`EngineInterface_FL.DrawDebugArc` _returnvalue (`self.maxRadius`) _returnvalue_2 10 (struct :`R` 1.0 :`G` 0.803995 :`A` 1.0) 0.0 0.0 _returnvalue_3))
          (:`then_1`
            (`EngineInterface_FL.DrawDebugArc` _returnvalue (`self.emergencyRadius`) _returnvalue_2 10 (struct :`R` 1.0 :`G` 0.133618 :`A` 1.0) 0.0 0.0 _returnvalue_3)))))
    (:`then_1`
      (if (`self.bDebugRays`)
        (`self.DebugRays`)))))

(fn `DebugRays`
  (locals (Loc :type "Vector Structure") (Rot :type "Rotator Structure"))
  (bind _loc (`local.Loc`))
  (bind _emergencyradius (`self.emergencyRadius`))
  (set `local.Loc` (`self.K2_GetActorLocation`))
  (set `local.Rot` (`KismetMathLibrary.ComposeRotators` (`self.K2_GetActorRotation`) (`KismetMathLibrary.NegateRotator` (`KismetMathLibrary.MakeRotator` 0.0 0.0 (+ (`self.halfAngle`) (.yaw (`self.deltaRotation`)))))))
  (for _ (range (+ (`self.rayCount`) 1))
    (bind _output_get (set `local.Rot` (`KismetMathLibrary.MakeRotator` 0.0 0.0 (+ (.yaw (`local.Rot`)) (.yaw (`self.deltaRotation`))))))
    (`|ExecutionSequence`
      (:`then_0`
        (bind _returnvalue (`KismetMathLibrary.GetForwardVector` _output_get))
        (bind _returnvalue_2 (+ _loc (* _returnvalue _emergencyradius)))
        (`KismetSystemLibrary.DrawDebugLine` _loc _returnvalue_2 (struct :`R` 1.0 :`G` 0.133618 :`A` 1.0)))
      (:`then_1`
        (`KismetSystemLibrary.DrawDebugLine` _returnvalue_2 (+ _loc (* _returnvalue (- (`self.maxRadius`) _emergencyradius))) (struct :`R` 1.0 :`G` 0.803995 :`A` 1.0))))))

(fn `UserConstructionScript`)