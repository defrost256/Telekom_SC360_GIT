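; BP_ParkingSlotDebug is a debug visualizer for a traffic parking slot, drawing colored points after each traffic tick.
; A large point at the slot, lifted by a signal offset, shows red when a car is assigned and green when free.
; For assigned cars, a small point marks the first spline point while arriving or the second while parking.
; It turns red when the car can start parking or leave the road, respectively, otherwise green.
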(event `self.AfterTrafficTick`
  (params (DeltaT :type "Float (single-precision)"))
  (bind _dotsizesmall (`self.DotSizeSmall`))
  (bind _dotsizesmall_2 (`self.DotSizeSmall`))
  (bind _returnvalue (+ (`SplineComponent.GetLocationAtSplinePoint` (`self.spline`) 0 "World") (`self.SignalOffset`)))
  (bind _returnvalue_2 (+ (`SplineComponent.GetLocationAtSplinePoint` (`self.spline`) 1 "World") (`self.SignalOffset`)))
  (if (`self.HasCar`)
    (`|ExecutionSequence`
      (:`then_0`
        ;[1 1 1] Assigned slot
        (`KismetSystemLibrary.DrawDebugPoint` (+ (`self.K2_GetActorLocation`) (`self.SignalOffset`)) (`self.DotSizeBig`) (struct :`R` 1.0 :`A` 1.0)))
      (:`then_1`
        (switch `EParkingState` (`self.state`)
          (:`Arriving`
            ;[1 1 1] Arriving
            (if (`self.CanCarStartParking`)
              (`KismetSystemLibrary.DrawDebugPoint` _returnvalue _dotsizesmall_2 (struct :`R` 1.0 :`A` 1.0))
              (else
                (`KismetSystemLibrary.DrawDebugPoint` _returnvalue _dotsizesmall_2 (struct :`G` 1.0 :`A` 1.0)))))
          (:`Parking`
            ;[1 1 1] Parking
            (if (`self.CanLeaveRoad` (`TrafficCar.time` (`|GetArrayItem` (`self.currentCars`))))
              (`KismetSystemLibrary.DrawDebugPoint` _returnvalue_2 _dotsizesmall (struct :`R` 1.0 :`A` 1.0))
              (else
                (`KismetSystemLibrary.DrawDebugPoint` _returnvalue_2 _dotsizesmall (struct :`G` 1.0 :`A` 1.0))))))))
    (else
      ;[1 1 1] Free slot
      (`KismetSystemLibrary.DrawDebugPoint` (+ (`self.K2_GetActorLocation`) (`self.SignalOffset`)) (`self.DotSizeBig`) (struct :`G` 1.0 :`A` 1.0)))))

(fn `UserConstructionScript`)