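; Canvas-drawn dashboard display for the saloon car, showing gear, speed in km/h and RPM over a background texture.
; An Interface event stores incoming speed, RPM, gear and texture values, which the Update event draws onto the canvas.
; Gear shows as R in red, N or a number; speed and RPM shift left by digit count to stay aligned, with RPM blank at zero.
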(event `self.ReceiveUpdate`
  (params (Canvas :type "Canvas Object Reference") (Width :type Integer) (Height :type Integer))
  (bind _gear (`self.Gear`))
  (bind _speed_x (`self.speed_x`))
  (bind _rpm_x (`self.RPM_x`))
  (bind _returnvalue (`KismetMathLibrary.FFloor` (`self.RPM`)))
  (bind _returnvalue_2 (`KismetMathLibrary.FFloor` (`self.Speed`)))
  (bind _returnvalue_3 (< _gear 0))
  (bind _returnvalue_4 (- _speed_x 20.0))
  (bind _returnvalue_5 (- _rpm_x 10.0))
  (bind _returnvalue_6 (> _returnvalue 0))
  (bind _returnvalue_7 (- _returnvalue_5 10.0))
  (`Canvas.K2_DrawTexture` Canvas (`self.Dash Texture`) (0.0 0.0) (1024.0 1024.0) (0.0 0.0) (1.0 1.0) (struct :`R` 1.0 :`G` 1.0 :`B` 1.0 :`A` 1.0) "BLEND_Opaque" 0.0 (0.5 0.5))
  (`Canvas.K2_DrawText` Canvas "/Game/PolymodelsCarsV01/Fonts/f_002_saloon_f_big.f_002_saloon_f_big" (`KismetMathLibrary.SelectString` "R" (`KismetMathLibrary.SelectString` "N" (`KismetStringLibrary.Conv_IntToString` _gear) (== _gear 0)) _returnvalue_3) (470.0 590.0) (`KismetMathLibrary.SelectColor` (struct :`R` 1.0 :`A` 1.0) (struct :`R` 0.75 :`G` 0.75 :`B` 0.75 :`A` 1.0) _returnvalue_3) 0.0 (struct :`A` 1.0) (1.0 1.0) false false false (struct :`A` 1.0))
  (`Canvas.K2_DrawText` Canvas "/Game/PolymodelsCarsV01/Fonts/f_002_saloon_f_small.f_002_saloon_f_small" (`KismetStringLibrary.BuildString_Int` "" "" _returnvalue_2 "km/h") (`KismetMathLibrary.MakeVector2D` (`KismetMathLibrary.SelectFloat` (- _returnvalue_4 5.0) (`KismetMathLibrary.SelectFloat` _returnvalue_4 _speed_x (> _returnvalue_2 9)) (> _returnvalue_2 99)) 950.0) (struct :`R` 0.75 :`G` 0.75 :`B` 0.75 :`A` 1.0) 0.0 (struct :`A` 1.0) (1.0 1.0) false false false (struct :`A` 1.0))
  (`Canvas.K2_DrawText` Canvas "/Game/PolymodelsCarsV01/Fonts/f_002_saloon_f_small.f_002_saloon_f_small" (`KismetMathLibrary.SelectString` (`KismetStringLibrary.BuildString_Int` "" "" _returnvalue) "" _returnvalue_6) (`KismetMathLibrary.MakeVector2D` (`KismetMathLibrary.SelectFloat` (- _returnvalue_7 10.0) (`KismetMathLibrary.SelectFloat` _returnvalue_7 (`KismetMathLibrary.SelectFloat` _returnvalue_5 (`KismetMathLibrary.SelectFloat` _rpm_x 0.0 _returnvalue_6) (> _returnvalue 9)) (> _returnvalue 99)) (> _returnvalue 999)) 885.0) (struct :`R` 0.75 :`G` 0.75 :`B` 0.75 :`A` 1.0) 0.0 (struct :`A` 1.0) (1.0 1.0) false false false (struct :`A` 1.0)))

(event `/Game/PolymodelsCarsV01/Blueprints/002_saloon_BPI.Interface`
  (params (`Steering Angle` :type "Float (single-precision)") (Speed :type "Float (single-precision)") (RPM :type "Float (single-precision)") (Gear :type Integer) (Left :type "Transform Structure") (Right :type "Transform Structure") (`Dash Texture` :type "Texture Object Reference") (roll :type "Float (single-precision)") (`Body Texture` :type "Texture Object Reference") (`Registration Number` :type String) (`Plate X` :type Integer) (`Plate Y` :type Integer))
  (set `self.Speed` Speed)
  (set `self.RPM` RPM)
  (set `self.Gear` Gear)
  (set `self.Dash Texture` `Dash Texture`))