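; Configurable SUV car prop whose look is built entirely in the construction script, with no runtime logic.
; A DoOnce sets the mesh and creates dynamic materials for body, glass, lights, interior and rear-view mirror, sharing some across slots.
; Exposed variables then drive paint, rust, decal, interior colours, plate text, lamp glow and headlight spotlight intensity.
; Optional cube and 2D scene captures render to textures for body/glass reflections and the mirror.
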(fn `UserConstructionScript`
  (`|ExecutionSequence`
    (:`then_0`
      (`/Engine/EditorBlueprintResources/StandardMacros.DoOnce` false
        (:`Completed`
          (`|ExecutionSequence`
            (:`then_0`
              (`StaticMeshComponent.SetStaticMesh` (`self.Mesh`) "/Game/PolymodelsCarsV01/Meshes/007_suv_SM.007_suv_SM"))
            (:`then_1`
              (bind _returnvalue (`PrimitiveComponent.CreateDynamicMaterialInstance` (`self.Mesh`) 0 (`PrimitiveComponent.GetMaterial` (`self.Mesh`) 0)))
              (set `self.Body Material` _returnvalue)
              (`PrimitiveComponent.SetMaterial` (`self.Mesh`) 0 (`self.Body Material`))
              (`PrimitiveComponent.SetMaterial` (`self.Mesh`) 7 (`self.Body Material`))
              (`PrimitiveComponent.SetMaterial` (`self.Mesh`) 13 (`self.Body Material`))
              (bind _returnvalue_2 (`PrimitiveComponent.CreateDynamicMaterialInstance` (`self.Mesh`) 1 (`PrimitiveComponent.GetMaterial` (`self.Mesh`) 1)))
              (set `self.Glass Material` _returnvalue_2)
              (bind _returnvalue_3 (`PrimitiveComponent.CreateDynamicMaterialInstance` (`self.Mesh`) 3 (`PrimitiveComponent.GetMaterial` (`self.Mesh`) 3)))
              (set `self.Lights Material` _returnvalue_3)
              (`PrimitiveComponent.SetMaterial` (`self.Mesh`) 3 (`self.Lights Material`))
              (`PrimitiveComponent.SetMaterial` (`self.Mesh`) 10 (`self.Lights Material`))
              (`PrimitiveComponent.SetMaterial` (`self.Mesh`) 16 (`self.Lights Material`))
              (bind _returnvalue_4 (`PrimitiveComponent.CreateDynamicMaterialInstance` (`self.Mesh`) 4 (`PrimitiveComponent.GetMaterial` (`self.Mesh`) 4)))
              (set `self.Interior Material` _returnvalue_4)
              (bind _returnvalue_5 (`PrimitiveComponent.CreateDynamicMaterialInstance` (`self.Mesh`) 5 "/Game/PolymodelsCarsV01/Materials/mi_001_sedan_rear_mirror.mi_001_sedan_rear_mirror"))
              (set `self.Rear View Mirror Material` _returnvalue_5))))))
    (:`then_1`
      (`|ExecutionSequence`
        (:`then_1`
          (`MaterialInstanceDynamic.SetScalarParameterValue` (`self.Body Material`) "body metallic" (`self.Body Metallic`))
          (`MaterialInstanceDynamic.SetScalarParameterValue` (`self.Body Material`) "body roughness" (`self.Body Roughness`))
          (`MaterialInstanceDynamic.SetVectorParameterValue` (`self.Body Material`) "body colour" (`self.Body Colour`))
          (`MaterialInstanceDynamic.SetScalarParameterValue` (`self.Body Material`) "body specular" (`self.Body Specular`))
          (`MaterialInstanceDynamic.SetScalarParameterValue` (`self.Body Material`) "body reflection" (`self.Body Reflection Amount`))
          (`MaterialInstanceDynamic.SetTextureParameterValue` (`self.Body Material`) "reflection texture" (`self.Body Reflection Texture`))
          (`MaterialInstanceDynamic.SetTextureParameterValue` (`self.Glass Material`) "reflection texture" (`self.Body Reflection Texture`))
          (`MaterialInstanceDynamic.SetScalarParameterValue` (`self.Body Material`) "rust amount" (`self.Rust Amount`))
          (`MaterialInstanceDynamic.SetVectorParameterValue` (`self.Body Material`) "rust colour" (`self.Rust Colour`))
          (`MaterialInstanceDynamic.SetTextureParameterValue` (`self.Body Material`) "decal texture" (`self.Decal Texture`)))
        (:`then_2`
          (`MaterialInstanceDynamic.SetScalarParameterValue` (`self.Lights Material`) "headlight" (`KismetMathLibrary.SelectFloat` (`self.Light Multiplier`) 0.0 (`self.Head Light`)))
          (`MaterialInstanceDynamic.SetScalarParameterValue` (`self.Lights Material`) "reverse" (`KismetMathLibrary.SelectFloat` (`self.Light Multiplier`) 0.0 (`self.Reverse`)))
          (`MaterialInstanceDynamic.SetScalarParameterValue` (`self.Lights Material`) "stop" (`KismetMathLibrary.SelectFloat` (`self.Light Multiplier`) 0.0 (`self.Stop`)))
          (`MaterialInstanceDynamic.SetScalarParameterValue` (`self.Lights Material`) "left" (`KismetMathLibrary.SelectFloat` (`self.Light Multiplier`) 0.0 (`self.Left`)))
          (`MaterialInstanceDynamic.SetScalarParameterValue` (`self.Lights Material`) "right" (`KismetMathLibrary.SelectFloat` (`self.Light Multiplier`) 0.0 (`self.Right`))))
        (:`then_3`
          (`LightComponent.SetIntensity` (`self.SpotLightRight`) (`KismetMathLibrary.SelectFloat` (* (`self.Light Multiplier`) 50.0) 0.0 (`self.Head Light`)))
          (`LightComponent.SetIntensity` (`self.SpotLightLeft`) (`KismetMathLibrary.SelectFloat` (* (`self.Light Multiplier`) 50.0) 0.0 (`self.Head Light`))))
        (:`then_4`
          (if (`self.Activate Body Reflections Camera?`)
            (bind _returnvalue_6 (`AddComponent|NODE_AddSceneCaptureComponentCube-0` :`RelativeTransform` (`KismetMathLibrary.MakeTransform` (0.0 0.0 167.0) (struct))))
            (set `self.Body Reflections Camera` _returnvalue_6)
            (set `SceneCaptureComponentCube.TextureTarget` (`self.Body Reflection Texture`) (`self.Body Reflections Camera`))
            (`MaterialInstanceDynamic.SetTextureParameterValue` (`self.Body Material`) "reflection texture" (`self.Body Reflection Texture`))
            (`MaterialInstanceDynamic.SetTextureParameterValue` (`self.Glass Material`) "reflection texture" (`self.Body Reflection Texture`))))
        (:`then_5`
          (`/Engine/EditorBlueprintResources/StandardMacros.IsValid` (`self.Rear Mirror Reflection Texture`)
            (:`Is Valid`
              (bind _returnvalue_7 (`AddComponent|NODE_AddSceneCaptureComponent2D-0` :`RelativeTransform` (`KismetMathLibrary.MakeTransform` (-212.0 0.0 31.0) (struct :`Yaw` 180.0))))
              (set `self.Rear View Mirror Camera` _returnvalue_7)
              (set `SceneCaptureComponent2D.TextureTarget` (`self.Rear Mirror Reflection Texture`) (`self.Rear View Mirror Camera`))
              (`MaterialInstanceDynamic.SetTextureParameterValue` (`self.Rear View Mirror Material`) "reflection texture" (`self.Rear Mirror Reflection Texture`)))))
        (:`then_6`
          (`TextRenderComponent.SetText` (`self.Front Plate`) (`self.Registration Plate`))
          (`TextRenderComponent.SetText` (`self.Rear Plate`) (`self.Registration Plate`)))
        (:`then_7`
          (`MaterialInstanceDynamic.SetVectorParameterValue` (`self.Interior Material`) "top colour" (`self.Top Colour`))
          (`MaterialInstanceDynamic.SetVectorParameterValue` (`self.Interior Material`) "plastic colour" (`self.Plastic Colour`))
          (`MaterialInstanceDynamic.SetVectorParameterValue` (`self.Interior Material`) "upholstery colour" (`self.Upholstery Colour`)))))))