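; RoadSpline_BP is a spline-driven road prop that builds itself in its Construction Script.
; It adds a deformed spline mesh per segment, with configurable width, collision and loop closure, and a dynamic material scaling texture by segment length.
; It also places a text label above each spline point.
; Optional pillars, built once via DoOnce, repeat at set spacing where the spline is high enough, stretching a column between lower and upper bases.
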(fn `UserConstructionScript`
  (bind _distance_between_pillars (`self.Distance Between Pillars`))
  (bind _spline (`self.Spline`))
  (bind _mesh_scale (`self.Mesh Scale`))
  (bind _index (`self.index`))
  (bind (_locallocation _localtangent) (`SplineComponent.GetLocalLocationAndTangentAtSplinePoint` (`self.Spline`) (`self.index`)))
  (bind _returnvalue (`KismetMathLibrary.MakeVector2D` (`self.Mesh Scale`) 1.0))
  (bind _returnvalue_2 (`KismetMathLibrary.MakeVector` 1.0 _mesh_scale 1.0))
  (bind (_locallocation_2 _localtangent_2) (`SplineComponent.GetLocalLocationAndTangentAtSplinePoint` (`self.index`)))
  (bind (_locallocation_3 _localtangent_3) (`SplineComponent.GetLocalLocationAndTangentAtSplinePoint` (+ (`self.index`) 1)))
  (for _index_2 (range (`SplineComponent.GetNumberOfSplinePoints`))
    (set `self.index` _index_2)
    (`|ExecutionSequence`
      (:`then_1`
        (bind _returnvalue_3 (`AddComponent|NODE_AddSplineMeshComponent-0` :`bManualAttachment` true))
        (set `self.MeshComponent` _returnvalue_3)
        (`SceneComponent.K2_AttachTo` (`self.MeshComponent`) (`self.Spline`) "None" "KeepRelativeOffset" true)
        (`SplineMeshComponent.SetStartAndEnd` (`self.MeshComponent`) _locallocation_2 _localtangent_2 _locallocation_3 _localtangent_3 true)
        (if (< (+ (`self.index`) 2) (`SplineComponent.GetNumberOfSplinePoints`))
          (set `self.SegmentLength` (`KismetMathLibrary.FFloor` (`KismetMathLibrary.Abs` (- (`SplineComponent.GetDistanceAlongSplineAtSplinePoint` (`self.Spline`) (+ _index 1)) (`SplineComponent.GetDistanceAlongSplineAtSplinePoint` (`self.Spline`) _index)))))))
      (:`then_2`
        (bind _returnvalue_4 (`KismetMaterialLibrary.CreateDynamicMaterialInstance` "/Game/PolymodelsCarsV01/Props/Materials/mi_road.mi_road"))
        (set `self.road material` _returnvalue_4)
        (`SplineMeshComponent.SetStartScale` (`self.MeshComponent`) _returnvalue true)
        (`SplineMeshComponent.SetEndScale` (`self.MeshComponent`) _returnvalue true)
        (`PrimitiveComponent.SetMaterial` (`self.MeshComponent`) 0 (`self.road material`))
        (`MaterialInstanceDynamic.SetScalarParameterValue` (`self.road material`) "scale x" (/ (`self.scale texture`) (`KismetMathLibrary.Conv_IntToDouble` (`self.SegmentLength`)))))
      (:`then_3`
        (`PrimitiveComponent.SetCollisionEnabled` (`self.MeshComponent`) (select `bool` (`self.Collision`) :`false` "NoCollision" :`true` "QueryAndPhysics" :!type "ECollisionEnabled Enum"))
        (`SplineComponent.SetClosedLoop` (`self.Spline`) (select `bool` (`self.closed`) :`true` true) true))
      (:`then_4`
        (bind _returnvalue_5 (`AddComponent|NODE_AddTextRenderComponent-0` :`RelativeTransform` (`KismetMathLibrary.MakeTransform` (`KismetMathLibrary.MakeVector` (.x _locallocation) (.y _locallocation) (+ (.z _locallocation) 50.0)) (`KismetMathLibrary.Conv_VectorToRotator` (* _localtangent -1.0)))))
        (`TextRenderComponent.SetText` _returnvalue_5 (`self.TextToRender`)))
      (:`then_5`
        (if (`self.MakeColumn?`)
          (`/Engine/EditorBlueprintResources/StandardMacros.DoOnce` false
            (:`Completed`
              (for _index_3 (range (+ (`.ReturnValue` (`KismetMathLibrary.FMod` (`SplineComponent.GetSplineLength` (`self.Spline`)) _distance_between_pillars)) 1))
                (bind _returnvalue_6 (* (`KismetMathLibrary.Conv_IntToDouble` _index_3) _distance_between_pillars))
                (bind _returnvalue_7 (`SplineComponent.GetWorldRotationAtDistanceAlongSpline` _spline _returnvalue_6))
                (bind _x (.x (.location (`KismetMathLibrary.MakeTransform` (- (`SplineComponent.GetWorldLocationAtDistanceAlongSpline` _spline _returnvalue_6) (`SceneComponent.K2_GetComponentLocation` _spline)) _returnvalue_7))))
                (bind _y (.y (.location (`KismetMathLibrary.MakeTransform` (- (`SplineComponent.GetWorldLocationAtDistanceAlongSpline` _spline _returnvalue_6) (`SceneComponent.K2_GetComponentLocation` _spline)) _returnvalue_7))))
                (bind _z (.z (.location (`KismetMathLibrary.MakeTransform` (- (`SplineComponent.GetWorldLocationAtDistanceAlongSpline` _spline _returnvalue_6) (`SceneComponent.K2_GetComponentLocation` _spline)) _returnvalue_7))))
                (if (> _z 300.0)
                  (bind _returnvalue_8 (`KismetMathLibrary.MakeRotator` 0.0 0.0 (.yaw _returnvalue_7)))
                  (bind _returnvalue_9 (`AddComponent|NODE_AddStaticMeshComponent-0` :`RelativeTransform` (`KismetMathLibrary.MakeTransform` (`KismetMathLibrary.MakeVector` _x _y 0.0) _returnvalue_8 _returnvalue_2)))
                  (`StaticMeshComponent.SetStaticMesh` _returnvalue_9 "/Game/PolymodelsCarsV01/Props/Meshes/low_base_SM.low_base_SM")
                  (bind _returnvalue_10 (`AddComponent|NODE_AddStaticMeshComponent-1` :`RelativeTransform` (`KismetMathLibrary.MakeTransform` (`KismetMathLibrary.MakeVector` _x _y 100.0) _returnvalue_8 (`KismetMathLibrary.MakeVector` 1.0 _mesh_scale (/ (- _z 150.0) 100.0)))))
                  (`StaticMeshComponent.SetStaticMesh` _returnvalue_10 "/Game/PolymodelsCarsV01/Props/Meshes/column_SM.column_SM")
                  (bind _returnvalue_11 (`AddComponent|NODE_AddStaticMeshComponent-2` :`RelativeTransform` (`KismetMathLibrary.MakeTransform` (`KismetMathLibrary.MakeVector` _x _y (- _z 150.0)) _returnvalue_8 _returnvalue_2)))
                  (`StaticMeshComponent.SetStaticMesh` _returnvalue_11 "/Game/PolymodelsCarsV01/Props/Meshes/upeer_base.upeer_base"))))))))))