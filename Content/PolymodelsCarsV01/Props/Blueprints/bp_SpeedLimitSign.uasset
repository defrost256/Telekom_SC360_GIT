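; Speed limit sign prop, pairing a sign mesh with a box trigger volume.
; The construction script applies variables for the sign's visibility, world yaw, relative location and optional mesh override, and sizes the box.
; The event graph holds only disabled stubs, so this Blueprint defines no overlap or runtime behavior.
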(fn `UserConstructionScript`
  (bind _show_sign (`self.Show Sign`))
  (`SceneComponent.SetVisibility` (`self.SpeedSign`) _show_sign false)
  (`SceneComponent.SetHiddenInGame` (`self.SpeedSign`) (not _show_sign) false)
  (`SceneComponent.K2_SetWorldRotation` (`self.SpeedSign`) (`KismetMathLibrary.MakeRotator` 0.0 0.0 (`self.sign Rotation`)) false false)
  (`SceneComponent.K2_SetRelativeLocation` (`self.SpeedSign`) (`self.Sign Location`) false true)
  (`BoxComponent.SetBoxExtent` (`self.Box`) (`self.Trigger Size`) true)
  (if (!= (`self.Sign Override`) null)
    (`StaticMeshComponent.SetStaticMesh` (`self.SpeedSign`) (`self.Sign Override`))))